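; FinishLine actor that ends a driving game with a win when an actor overlaps it and TotalCollision is at least four.
; It sets GameWon before casting to SportsCar_Pawn; a successful cast shows WB_GameWin, pauses the game and switches to UI-only input with the cursor.
; Unconnected leftover nodes would count CanFinish flags from a BP_Collision actor, so nothing in this graph actually increments TotalCollision.
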(event Collision|EventActorBeginOverlap
  (params (OtherActor :type Actor%20Object%20Reference))
  (bind _returnvalue (Game|GetPlayerController 0))
  (if (>= (Variables|Default|GetTotalCollision) 4)
    (Variables|Default|SetGameWon true)
    (Utilities|Casting|CastToSportsCar_Pawn OtherActor)
    (bind _returnvalue_2 (UserInterface|CreateWidget "/Game/Blueprints/WB_GameWin.WB_GameWin_C"))
    (UserInterface|Viewport|AddtoViewport _returnvalue_2 0)
    (Variables|/Script/Engine.PlayerController|SetbShowMouseCursor _returnvalue true)
    (Game|SetGamePaused true)
    (Input|SetInputModeUIOnly _returnvalue _returnvalue_2 "DoNotLock" false)))

(event EventTick
  (params (DeltaSeconds :type Float%20%28single-precision%29)))

(fn ConstructionScript)