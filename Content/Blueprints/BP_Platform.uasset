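; BP_Platform runs the level countdown and triggers the lose screen when time runs out.
; BeginPlay caches the first FinishLine actor to read its GameWon flag.
; Tick gates on a one-second Delay to decrement Minutes and Seconds, and stalls on a very long Delay once won.
; At expiry without a win, it shows the WB_GameLose widget, pauses the game and switches to UI-only input with the cursor visible.
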(event EventBeginPlay
  (bind _outactors (Actor|GetAllActorsOfClass "/Game/Blueprints/FinishLine.FinishLine_C"))
  (Variables|Default|SetNewVar_0 (Utilities|Array|Get(acopy) _outactors)))

(event Collision|EventActorBeginOverlap
  (params (OtherActor :type Actor%20Object%20Reference)))

(event EventTick
  (params (DeltaSeconds :type Float%20%28single-precision%29))
  (bind _returnvalue (Game|GetPlayerController 0))
  (Utilities|FlowControl|Delay 1.0)
  (if (Variables|/Game/Blueprints/FinishLine.FinishLine_C|GetGameWon (Variables|Default|GetNewVar_0))
    (Utilities|FlowControl|Delay 1e+06)
    (elif (== (Variables|Default|GetSeconds) 1)
      (if (== (Variables|Default|GetMinutes) 0)
        (if (not (Variables|/Game/Blueprints/FinishLine.FinishLine_C|GetGameWon (Variables|Default|GetNewVar_0)))
          (bind _returnvalue_2 (UserInterface|CreateWidget "/Game/Blueprints/WB_GameLose.WB_GameLose_C"))
          (UserInterface|Viewport|AddtoViewport _returnvalue_2 0)
          (Variables|/Script/Engine.PlayerController|SetbShowMouseCursor _returnvalue true)
          (Game|SetGamePaused true)
          (Input|SetInputModeUIOnly _returnvalue _returnvalue_2 "DoNotLock" false)
          (Utilities|FlowControl|Delay 1e+06))
        (else
          (Variables|Default|SetSeconds 59)
          (Variables|Default|SetMinutes (- (Variables|Default|GetMinutes) 1))))
      (else
        (Variables|Default|SetSeconds (- (Variables|Default|GetSeconds) 1))))))

(fn ConstructionScript)