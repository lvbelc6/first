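; BP_Collision is a trigger actor that reports overlaps to the level's FinishLine actor.
; On any actor overlap, it looks up all FinishLine actors and increments TotalCollision on the first, with no filter or repeat guard.
; An unconnected leftover chain, which never runs, marks CanFinish array entries, advances an index and prints its own collision count.
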(event EventBeginPlay)

(event Collision|EventActorBeginOverlap
  (params (OtherActor :type Actor%20Object%20Reference))
  (bind _outactors (Actor|GetAllActorsOfClass "/Game/Blueprints/FinishLine.FinishLine_C"))
  (Variables|Default|SetNewVar_0 (Utilities|Array|Get(acopy) _outactors))
  (Math|Integer|IncrementInt (Variables|/Game/Blueprints/FinishLine.FinishLine_C|GetTotalCollision (Variables|Default|GetNewVar_0))))

(event EventTick
  (params (DeltaSeconds :type Float%20%28single-precision%29)))

(fn ConstructionScript)